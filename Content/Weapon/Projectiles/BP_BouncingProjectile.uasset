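; BP_BouncingProjectile is a player ability projectile that bounces between nearby pawns and shortens the player's other ability cooldowns.
; On overlap it sphere-traces for another pawn, ignoring the player, current and previous targets, then redirects its velocity toward it.
; Each successful bounce uses GAS cooldown tags to reduce active cooldowns, excluding the Skill1 cooldown, which must be active.
; It destroys itself when no target is found or the bounce limit is exceeded.
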(event EventOnCapsuleBeginOverlap
  (params (OverlappedComponent :type Primitive%20Component%20Object%20Reference) (OtherActor :type Actor%20Object%20Reference) (OtherComponent :type Primitive%20Component%20Object%20Reference) (OtherBodyIndex :type Integer) (bFromSweep :type Boolean) (SweepResult :type Hit%20Result%20Structure%20%28by%20ref%29))
  (|CallParentFunction OverlappedComponent OtherActor OtherComponent OtherBodyIndex bFromSweep SweepResult)
  (if (<= (Variables|Private|GetCurrentBounceCount) (Variables|Default|GetMaxBounceNumber))
    (Math|Integer|IncrementInt (Variables|Private|GetCurrentBounceCount)
      (:%20%20
        (bind _bsuccess (CallFunction|TryFindNextActor OtherActor))
        (if _bsuccess
          (CallFunction|ReduceAbilitiesCooldown)
          (else
            (Actor|DestroyActor)))))
    (else
      (Actor|DestroyActor))))

(event EventBeginPlay
  (bind _asbp_player_character (Utilities|Casting|CastToBP_PlayerCharacter (Components|GetOwner)))
  (Variables|Private|SetPlayer _asbp_player_character))

(fn ConstructionScript)

(fn SetVelocity
  (params (TargetLocation :type Vector))
  (Variables|/Script/Engine.MovementComponent|SetVelocity (Variables|Default|GetProjectileMovementComponent) (* (Math|Vector|GetUnitDirection(Vector) (Transformation|GetActorLocation) TargetLocation) (Variables|/Script/Engine.ProjectileMovementComponent|GetInitialSpeed (Variables|Default|GetProjectileMovementComponent)))))

(fn TryFindNextActor
  (params (OtherActor :type Actor%20Object%20Reference))
  (bind _returnvalue (Transformation|GetActorLocation))
  (LocalVariables|SetLOCAL_OtherActor OtherActor)
  (bind (_outhit _returnvalue_2) (Collision|SphereTraceForObjects _returnvalue _returnvalue (Variables|Default|GetActorsSearchRadius) (Utilities|Array|MakeArray "ObjectTypeQuery3") false (Utilities|Array|MakeArray (LocalVariables|GetLOCAL_OtherActor) (Game|GetPlayerCharacter 0) (Variables|Private|GetPreviousAffectedActor)) "ForDuration"))
  (if _returnvalue_2
    (Variables|Private|SetPreviousAffectedActor (LocalVariables|GetLOCAL_OtherActor))
    (CallFunction|SetVelocity (Transformation|GetActorLocation (.HitActor (Collision|BreakHitResult _outhit))))
    (return true)
    (else
      (return false))))

(fn ReduceAbilitiesCooldown
  (bind _returnvalue (GameplayEffects|GetActiveEffectswithAllTags (Variables|/Script/Test.GASCharacter|GetAbilitySystemComponent (Variables|Private|GetPlayer)) "(GameplayTags=((TagName=\"Ability.Cooldown.Skill1\")))"))
  (if (> (Utilities|Array|Length _returnvalue) 0)
    (LocalVariables|SetLOCAL_BoucingProjectileActiveCD (Utilities|Array|Get(acopy) _returnvalue))
    (bind _returnvalue_2 (GameplayEffects|GetActiveEffectswithAllTags (Variables|/Script/Test.GASCharacter|GetAbilitySystemComponent (Variables|Private|GetPlayer)) "(GameplayTags=((TagName=\"Ability.Cooldown\")))"))
    (if (> (Utilities|Array|Length _returnvalue_2) 0)
      (for _array_element _returnvalue_2
        (if (!= _array_element (LocalVariables|GetLOCAL_BoucingProjectileActiveCD))
          (bind _returnvalue_3 (Ability|GameplayEffect|GetActiveGameplayEffectRemainingDuration _array_element))
          (Default|TrytoReduceAbilityCooldown (Variables|Private|GetPlayer) _array_element (- _returnvalue_3 (Variables|Default|GetCooldownDecreaseTime)))))
      (return)
      (else
        (return)))
    (else
      (return))))