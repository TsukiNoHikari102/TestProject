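; Player character Blueprint built on the Gameplay Ability System, with a HUD, an ability manager menu and skill-point ability upgrades.
; BeginPlay passes the AbilitySystemComponent to the HUD, while an Enhanced Input action opens the manager in UI-only mode.
; TryLevelUpAbility finds the granted spec by class and spends a point to raise its level; TryToReduceAbilityCooldown overrides an active effect's duration.
; Hard-wired keys open ThirdPersonMap and toggle ragdoll.
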(event EventBeginPlay
  (|CallParentFunction)
  (bind _returnvalue (UserInterface|CreateWidget "/Game/Core/UI/HUD/WBP_HUD.WBP_HUD_C" (Game|GetPlayerController 0) (Variables|Default|GetAbilitySystemComponent)))
  (bind _output_get (Variables|Widgets|SetWBP_HUD _returnvalue))
  (UserInterface|Viewport|AddtoViewport _output_get 0))

(event Input|EnhancedActionEvents|EnhancedInputActionIA_AbilityManager
  (params (ActionValue :type Boolean) (ElapsedSeconds :type Float%20%28double-precision%29) (TriggeredSeconds :type Float%20%28double-precision%29) (InputAction :type Input%20Action%20Object%20Reference :default "/Game/Core/Player/Input/Actions/IA_AbilityManager.IA_AbilityManager"))
  (bind _returnvalue (Game|GetPlayerController 0))
  (:Started
    (bind _returnvalue_2 (UserInterface|CreateWidget "/Game/Core/UI/HUD/WBP_AbilityManager.WBP_AbilityManager_C" (Game|GetPlayerController 0)))
    (bind _output_get (Variables|Widgets|SetWBP_AbilityManager _returnvalue_2))
    (UserInterface|Viewport|AddtoViewport _output_get 0)
    (Input|SetInputModeUIOnly _returnvalue _output_get "DoNotLock" false)
    (Variables|/Script/Engine.PlayerController|SetbShowMouseCursor _returnvalue true)))

(event Input|KeyboardEvents|3
  (params (Key :type Key%20Structure :default "None"))
  (:Pressed
    (Utilities|FlowControl|FlipFlop
      (:A
        (Class|GASCharacter|ApplyRagdoll))
      (:B
        (Class|GASCharacter|ExitRagdoll)))))

(event Input|KeyboardEvents|R
  (params (Key :type Key%20Structure :default "None"))
  (:Pressed
    (Game|OpenLevel(byName) "ThirdPersonMap")))

(event EventDamage
  (params (DamageInstigator :type GAS%20Character%20Object%20Reference) (Hit :type Hit%20Result%20Structure%20%28by%20ref%29) (Damage :type Float%20%28single-precision%29)))

(fn ConstructionScript)

(fn TryLevelUpAbility
  (params (AbilityInfo :type PDA%20Ability%20Info%20Object%20Reference))
  (if (> (Variables|Ability|GetSkillPoints) 0)
    (LocalVariables|SetLOCAL_AbilityInfo AbilityInfo)
    (bind _outabilityhandles (Class|AbilitySystemComponent|GetAllAbilities (Variables|Default|GetAbilitySystemComponent)))
    (bind _array_element (Utilities|Array|ForEachLoopwithBreak _outabilityhandles :!label _label)
      (:LoopBody
        (LocalVariables|SetLOCAL_AbilitySpecHandle _array_element)
        (Utilities|IsValid (.ReturnValue (Ability|GameplayAbility|GetGameplayAbilityfromSpecHandle (Variables|Default|GetAbilitySystemComponent) _array_element))
          (:Is%20Valid
            (if (== (Utilities|GetClass (.ReturnValue (Ability|GameplayAbility|GetGameplayAbilityfromSpecHandle (Variables|Default|GetAbilitySystemComponent) _array_element))) (Variables|/Script/TestProject.PDA_AbilityInfo|GetAbilityClass (LocalVariables|GetLOCAL_AbilityInfo)))
              (bind _output_get (LocalVariables|SetLOCAL_GameplayAbility (.ReturnValue (Ability|GameplayAbility|GetGameplayAbilityfromSpecHandle (Variables|Default|GetAbilitySystemComponent) _array_element))))
              (LocalVariables|SetLOCAL_AbilityLevel (Ability|GetAbilityLevel _output_get))
              (LocalVariables|SetLOCAL_bSameAbilityFound true)
              (goto _label Break)))))
      (:Completed
        (if (LocalVariables|GetLOCAL_bSameAbilityFound)
          (bind _ascore_gameplay_ability (Utilities|Casting|CastToCoreGameplayAbility (LocalVariables|GetLOCAL_GameplayAbility)))
          (Class|GASAbilitySystemComponent|SetAbilityLevel (Variables|Default|GetAbilitySystemComponent) (LocalVariables|GetLOCAL_AbilitySpecHandle) _ascore_gameplay_ability (+ (LocalVariables|GetLOCAL_AbilityLevel) 1))
          (bind _result (Math|Integer|DecrementInt (Variables|Ability|GetSkillPoints))
            (:%20%20
              (return true (+ (LocalVariables|GetLOCAL_AbilityLevel) 1) _result)))
          (else
            (return false 0 0)))))
    (else
      (Development|PrintString "You don't have enough skill points")
      (return false 0 0))))

(fn TrytoReduceAbilityCooldown
  (params (ActiveEffectHandle :type Active%20Gameplay%20Effect%20Handle%20Structure) (NewDuration :type Float%20%28double-precision%29))
  (bind _returnvalue (Class|GASAbilitySystemComponent|SetGameplayEffectDurationHandle (Variables|Default|GetAbilitySystemComponent) ActiveEffectHandle NewDuration))
  (return _returnvalue))