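; Player gameplay ability that reduces damage from projectiles striking the hit actor from the front.
; On a gameplay event with a projectile payload, it dots reversed impact velocity with the actor's forward vector against a level-based threshold.
; Frontal hits scale the instigator's base attribute value down by a level-based fraction.
; The result reaches the hit actor through BP_GE_GetDamage as SetByCaller magnitude; CheckAngle is an empty stub.
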(event Ability|EventActivateAbilityFromEvent
  (params (EventData :type Gameplay%20Event%20Data%20Structure%20%28by%20ref%29))
  (bind (_eventtag _instigator _target _optionalobject _optionalobject2 _contexthandle _instigatortags _targettags _eventmagnitude _targetdata) (Utilities|Struct|BreakGameplayEventData EventData))
  (bind _returnvalue (Ability|TargetData|GetHitResultfromTargetData _targetdata))
  (bind _returnvalue_2 (Ability|GetAbilitySystemComponent _instigator))
  (bind _returnvalue_3 (Class|AbilitySystemBlueprintLibrary|GetFloatAttributeBasefromAbilitySystemComponent _returnvalue_2 "(AttributeName=\"Damage\",Attribute=/Script/Test.CharacterAttributeSet:Damage,AttributeOwner=/Script/CoreUObject.Class'\"/Script/Test.CharacterAttributeSet\"')"))
  (bind _asabil_payload_projectile (Utilities|Casting|CastToAbilPayload_Projectile _optionalobject)
    (:then
      (bind _values (Utilities|Map|Values (.UpgradableParams (Utilities|Struct|BreakAbilityUpgradeStructure (Utilities|Array|Get(acopy) (Variables|/Script/Test.PDA_AbilityInfo|GetAbilityLevelingInfo (Variables|Default|GetAbilityData)) (- (Ability|GetAbilityLevel) 1))))))
      (if (> (Math|Vector|DotProduct (Math|Vector|Normalize (* (Variables|/Script/Test.AbilPayload_Projectile|GetImpactVelocity _asabil_payload_projectile) -1.0)) (Transformation|GetActorForwardVector (.hitactor _returnvalue))) (- 1.0 (/ (/ (Utilities|Array|Get(acopy) _values) 1e+02) 2.0)))
        (Variables|Default|SetDamage (* _returnvalue_3 (- 1.0 (Utilities|Array|Get(acopy) _values 1))))
        (else
          (Variables|Default|SetDamage _returnvalue_3)))
      (bind _returnvalue_4 (Ability|GameplayEffect|AssignTagSetbyCallerMagnitude (GameplayEffects|MakeOutgoingSpec :self (.abilitysystemcomponent (Ability|GetActorInfo)) :GameplayEffectClass "/Game/Core/GAS/GameplayEffects/Health/BP_GE_GetDamage.BP_GE_GetDamage_C" :Level 1.0) "(TagName=\"Attribute.BaseDamage\")" (Variables|Default|GetDamage)))
      (GameplayEffects|ApplyGameplayEffectSpecToTarget _returnvalue_4 (Ability|TargetData|AbilityTargetDatafromActor (.hitactor _returnvalue)))
      (Ability|EndAbility))
    (:CastFailed
      (Ability|CancelAbility))))

(fn CheckAngle
  (params (OptionalObject :type Object%20Object%20Reference)))