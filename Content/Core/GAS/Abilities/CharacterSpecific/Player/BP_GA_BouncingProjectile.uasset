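; Player gameplay ability that lets the character aim at an actor and fire a bouncing projectile at it.
; On activation it adjusts the camera boom for aiming, checks cooldown and cost, then awaits a user-confirmed sphere-trace target with a reticle.
; A valid actor target commits the ability and spawns BP_BouncingProjectile, configured from ability-level data and given the hit location.
; Ending the ability restores the saved camera settings.
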(event Ability|EventActivateAbility
  (CallFunction|SaveDefaultCameraParams)
  (CallFunction|SetNewCameraParams (+ (Variables|Private|GetCameraBoomDefaultRelativeLocation) "0.000000,0.000000,80.000000") (Variables|Default|GetAimingArmLength))
  (bind _returnvalue (Class|GameplayAbility|CheckAbilityCooldown))
  (bind _returnvalue_2 (Class|GameplayAbility|CheckAbilityCost))
  (if (and _returnvalue_2 _returnvalue)
    (bind _data (|WaitTargetData :ConfirmationType "UserConfirmed" :Class "/Script/Test.TargetActor_SphereTrace" :TraceSphereRadius 2e+01 :MaxRange 1e+04 :TraceProfile "(Name=\"IgnoreOnlyPawn\")" :bIgnoreBlockingHits false :bTraceFromPlayerViewPoint true :bUsePersistentHitResults true :StartLocation (CallFunction|SetupTargetLocationInfo) :ReticleClass "/Game/Core/GAS/ReticleClasses/BP_BouncingProjectileReticle.BP_BouncingProjectileReticle_C")
      (:ValidData
        (bind _output_get (Variables|Private|SetTargetData _data))
        (if (Ability|TargetData|TargetDataHasActor _output_get)
          (bind _returnvalue_3 (Ability|CommitAbility))
          (if _returnvalue_3
            (CallFunction|TrySpawnProjectile)
            (Ability|EndAbility)
            (else
              (Ability|CancelAbility :!label _label)))
          (else
            (goto _label))))
      (:Cancelled
        (Ability|CancelAbility)))
    (else
      (Ability|CancelAbility))))

(event Ability|EventOnEndAbility
  (params (bWasCancelled :type Boolean))
  (CallFunction|SetNewCameraParams (Variables|Private|GetCameraBoomDefaultRelativeLocation) (Variables|Private|GetCameraBoomDefaultArmLength)))

(fn SaveDefaultCameraParams
  (bind _asbp_player_character (Utilities|Casting|CastToBP_PlayerCharacter (Ability|GetAvatarActorfromActorInfo)))
  (bind _output_get (Variables|Private|SetAvatarActor _asbp_player_character))
  (Variables|Private|SetCameraBoomDefaultRelativeLocation (Variables|/Script/Engine.SceneComponent|GetRelativeLocation (Variables|/Script/Test.GASCharacter|GetCameraBoom _output_get)))
  (Variables|Private|SetCameraBoomDefaultArmLength (Variables|/Script/Engine.SpringArmComponent|GetTargetArmLength (Variables|/Script/Test.GASCharacter|GetCameraBoom _output_get))))

(fn SetNewCameraParams
  (params (NewLocation :type Vector) (NewArmLength :type Float%20%28single-precision%29))
  (bind _avataractor (Variables|Private|GetAvatarActor))
  (bind _cameraboom (Variables|/Script/Test.GASCharacter|GetCameraBoom _avataractor))
  (Transformation|SetRelativeLocation _cameraboom NewLocation false false)
  (Variables|/Script/Engine.SpringArmComponent|SetTargetArmLength _cameraboom NewArmLength))

(fn SetupTargetLocationInfo
  (bind _returnvalue (Class|GameplayAbility|MakeTargetLocationInfofromOwnerActor))
  (bind (_locationtype _literaltransform _sourceactor _sourcecomponent _sourceability _sourcesocketname) (Utilities|Struct|BreakGameplayAbilityTargetingLocationInfo _returnvalue))
  (return (Utilities|Struct|MakeGameplayAbilityTargetingLocationInfo _locationtype (Math|Transform|MakeTransform (+ (* (Transformation|GetActorForwardVector (Variables|Private|GetAvatarActor)) 2e+02) (.location _literaltransform)) (.rotation _literaltransform) (.scale _literaltransform)) _sourceactor _sourcecomponent _sourceability _sourcesocketname)))

(fn TrySpawnProjectile
  (bind _avataractor (Variables|Private|GetAvatarActor))
  (bind _values (Utilities|Map|Values (.UpgradableParams (Utilities|Struct|BreakAbilityUpgradeStructure (Utilities|Array|Get(acopy) (Variables|/Script/Test.PDA_AbilityInfo|GetAbilityLevelingInfo (Variables|Default|GetAbilityData)) (- (Ability|GetAbilityLevel) 1))))))
  (bind _returnvalue (Game|SpawnActorfromClass "/Game/Weapon/Projectiles/BP_BouncingProjectile.BP_BouncingProjectile_C" (Math|Transform|MakeTransform (+ (Transformation|GetActorLocation _avataractor) (Variables|Default|GetProjectileSpawnOffset)) (Transformation|GetActorRotation _avataractor) "1.000000,1.000000,1.000000") "AlwaysSpawn" "MultiplyWithRoot" _avataractor (Math|Float|Truncate (Utilities|Array|Get(acopy) _values)) (Utilities|Array|Get(acopy) _values 1) (Utilities|Array|Get(acopy) _values 2) 0))
  (Utilities|IsValid _returnvalue
    (:Is%20Valid
      (Default|SetVelocity _returnvalue (.location (Ability|TargetData|GetHitResultfromTargetData (Variables|Private|GetTargetData))))
      (return))
    (:Is%20Not%20Valid
      (return))))