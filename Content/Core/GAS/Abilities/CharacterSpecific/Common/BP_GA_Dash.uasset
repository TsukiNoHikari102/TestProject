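; Gameplay ability that dashes the avatar after a level-defined delay, granting invulnerability until it ends and damaging pawns along the way.
; Root-motion MoveTo carries it along its velocity, or forward when nearly still.
; A looping timer box-traces ahead during the move, applying SetByCaller damage once per actor via DamagedActors.
; Distance, delay and damage come from the ability level's upgradable params, read by index.
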(event Custom|StartDashing
  (bind _returnvalue (Ability|GetAvatarActorfromActorInfo))
  (bind _returnvalue_2 (Ability|GetAvatarActorfromActorInfo))
  (bind _returnvalue_3 (Transformation|GetVelocity _returnvalue))
  (Ability|ApplyGameplayEffectToOwner "/Game/Core/GAS/GameplayEffects/Common/BP_GE_Invulnerability.BP_GE_Invulnerability_C")
  (bind _values (Utilities|Map|Values (.UpgradableParams (Utilities|Struct|BreakAbilityUpgradeStructure (Utilities|Array|Get(acopy) (Variables|/Script/Test.PDA_AbilityInfo|GetAbilityLevelingInfo (Variables|Default|GetAbilityData)) (- (Ability|GetAbilityLevel) 1))))))
  (Variables|Default|SetDistance (Utilities|Array|Get(acopy) _values))
  (if (<= (Math|Vector|VectorLength _returnvalue_3) 5.0)
    (Ability|Tasks|ApplyRootMotionMoveToForce "None" (+ (Transformation|GetActorLocation _returnvalue_2) (* (Transformation|GetActorForwardVector _returnvalue_2) (Variables|Default|GetDistance))) 0.15 false "MOVE_None" false 0 "MaintainLastRootMotionVelocity"
      (:then
        (CallFunction|TryDamageEnemies)
        (bind _returnvalue_4 (Utilities|Time|SetTimerbyEvent (EventDispatchers|CreateEvent :!event TryDamageEnemies) 0.03 true))
        (Variables|Default|SetTryDamageTimerH _returnvalue_4))
      (:OnTimedOut
        (Utilities|Time|ClearandInvalidateTimerbyHandle (Variables|Default|GetTryDamageTimerH) :!label _label)
        (Utilities|Array|Clear (Variables|Default|GetDamagedActors))
        (Ability|EndAbility))
      (:OnTimedOutAndDestinationReached
        (goto _label)))
    (else
      (Ability|Tasks|ApplyRootMotionMoveToForce "None" (+ (Transformation|GetActorLocation _returnvalue) (* (Math|Vector|Normalize _returnvalue_3) (Variables|Default|GetDistance))) 0.15 false "MOVE_None" false 0 "MaintainLastRootMotionVelocity" _returnvalue_3
        (:then
          (CallFunction|TryDamageEnemies)
          (bind _returnvalue_5 (Utilities|Time|SetTimerbyEvent (EventDispatchers|CreateEvent :!event TryDamageEnemies) 0.03 true))
          (Variables|Default|SetTryDamageTimerH _returnvalue_5))
        (:OnTimedOut
          (goto _label))
        (:OnTimedOutAndDestinationReached
          (goto _label))))))

(event Ability|EventActivateAbility
  (bind _returnvalue (Ability|CommitAbility))
  (if _returnvalue
    (CallFunction|SetTimertoStartDashing)
    (else
      (Ability|CancelAbility))))

(event Ability|EventOnEndAbility
  (params (bWasCancelled :type Boolean))
  (Ability|RemoveGameplayEffectFromOwnerWithAssetTags "(GameplayTags=((TagName=\"Effect.Invulnerability\")))"))

(fn SetTimertoStartDashing
  (bind _values (Utilities|Map|Values (.UpgradableParams (Utilities|Struct|BreakAbilityUpgradeStructure (Utilities|Array|Get(acopy) (Variables|/Script/Test.PDA_AbilityInfo|GetAbilityLevelingInfo (Variables|Default|GetAbilityData)) (- (Ability|GetAbilityLevel) 1))))))
  (Utilities|Time|SetTimerbyEvent (EventDispatchers|CreateEvent :!event Custom|StartDashing) (Utilities|Array|Get(acopy) _values 1)))

(fn TryDamageEnemies
  (bind _returnvalue (Ability|GetAvatarActorfromActorInfo))
  (bind _returnvalue_2 (Transformation|GetActorLocation _returnvalue))
  (bind _returnvalue_3 (Transformation|GetActorForwardVector _returnvalue))
  (bind _returnvalue_4 (* _returnvalue_3 5e+01))
  (bind _returnvalue_5 (+ _returnvalue_2 _returnvalue_4))
  (bind _outhits (Class|KismetSystemLibrary|BoxTraceMultiforObjects _returnvalue_5 _returnvalue_5 "20.000000,40.000000,40.000000" (Transformation|GetActorRotation _returnvalue) (Utilities|Array|MakeArray "ObjectTypeQuery3") false (Variables|Default|GetDamagedActors) "None" true))
  (for _array_element _outhits
    (if (== (Utilities|Array|FindItem (Variables|Default|GetDamagedActors) (.HitActor (Collision|BreakHitResult _array_element))) -1)
      (Utilities|Array|AddUnique (Variables|Default|GetDamagedActors) (.HitActor (Collision|BreakHitResult _array_element)))
      (bind _values (Utilities|Map|Values (.UpgradableParams (Utilities|Struct|BreakAbilityUpgradeStructure (Utilities|Array|Get(acopy) (Variables|/Script/Test.PDA_AbilityInfo|GetAbilityLevelingInfo (Variables|Default|GetAbilityData)) (- (Ability|GetAbilityLevel) 1))))))
      (bind _returnvalue_6 (Ability|GameplayEffect|AssignTagSetbyCallerMagnitude (GameplayEffects|MakeOutgoingSpec :self (.abilitysystemcomponent (Ability|GetActorInfo)) :GameplayEffectClass "/Game/Core/GAS/GameplayEffects/Health/BP_GE_GetDamage.BP_GE_GetDamage_C" :Level 1.0) "(TagName=\"Attribute.BaseDamage\")" (Utilities|Array|Get(acopy) _values 2)))
      (GameplayEffects|ApplyGameplayEffectSpecToTarget _returnvalue_6 (Ability|TargetData|AbilityTargetDatafromActor (.HitActor (Collision|BreakHitResult _array_element)))))))