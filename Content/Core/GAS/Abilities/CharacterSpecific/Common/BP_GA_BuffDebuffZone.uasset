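; BP_GA_BuffDebuffZone is a gameplay ability that spawns an effect zone at the avatar character's feet.
; On activation it commits, or cancels if that fails, then spawns EffectZoneClass at the capsule's base.
; The zone's radius, lifetime, trigger interval, healing and damage come from AbilityData for the current level, read by position from the upgradable parameter values.
; The graph never calls EndAbility after a successful spawn.
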(event Ability|EventActivateAbility
  (bind _returnvalue (Ability|GetAvatarActorfromActorInfo))
  (bind _returnvalue_2 (Transformation|GetActorLocation _returnvalue))
  (bind _returnvalue_3 (Ability|CommitAbility))
  (if _returnvalue_3
    (bind _ascharacter (Utilities|Casting|CastToCharacter _returnvalue))
    (bind _values (Utilities|Map|Values (.UpgradableParams (Utilities|Struct|BreakAbilityUpgradeStructure (Utilities|Array|Get(acopy) (Variables|/Script/Test.PDA_AbilityInfo|GetAbilityLevelingInfo (Variables|Default|GetAbilityData)) (- (Ability|GetAbilityLevel) 1))))))
    (Game|SpawnActorfromClass (Variables|Default|GetEffectZoneClass) (Math|Transform|MakeTransform (Math|Vector|MakeVector (.x _returnvalue_2) (.y _returnvalue_2) (- (.z _returnvalue_2) (Components|Capsule|GetScaledCapsuleHalfHeight (Variables|/Script/Engine.Character|GetCapsuleComponent _ascharacter)))) "0, 0, 0" "1.000000,1.000000,1.000000") "AlwaysSpawn" "MultiplyWithRoot" 0 (Utilities|Array|Get(acopy) _values 3) (Utilities|Array|Get(acopy) _values 4) (Utilities|Array|Get(acopy) _values) (Utilities|Array|Get(acopy) _values 1) (Utilities|Array|Get(acopy) _values 2) 0)
    (else
      (Ability|CancelAbility))))