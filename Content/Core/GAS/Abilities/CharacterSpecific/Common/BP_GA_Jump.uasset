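; BP_GA_Jump is a Gameplay Ability that makes a GASCharacter jump.
; On activation it commits the ability, caches the avatar, binds to its landed delegate and calls Jump.
; A WaitInputRelease task calls StopJumping when input is released, so holding the input can affect the jump.
; The ability stays active until OnLanded unbinds the delegate and ends it.
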(event Custom|OnLanded
  (params (Hit :type Hit%20Result%20Structure%20%28by%20ref%29))
  (EventDispatchers|UnbindEventfromLandedDelegate (Variables|Default|GetAvatarActor) (EventDispatchers|CreateEvent :!event Custom|OnLanded))
  (Ability|EndAbility))

(event Ability|EventActivateAbility
  (bind _returnvalue (Ability|CommitAbility))
  (if _returnvalue
    (Utilities|FlowControl|Sequence
      (:then_0
        (bind _asgascharacter (Utilities|Casting|CastToGASCharacter (Ability|GetAvatarActorfromActorInfo)))
        (bind _output_get (Variables|Default|SetAvatarActor _asgascharacter))
        (EventDispatchers|BindEventtoLandedDelegate _output_get (EventDispatchers|CreateEvent :!event Custom|OnLanded)))
      (:then_1
        (Character|Jump (Variables|Default|GetAvatarActor)))
      (:then_2
        (Ability|Tasks|WaitInputRelease false
          (:OnRelease
            (Character|StopJumping (Variables|Default|GetAvatarActor))))))))