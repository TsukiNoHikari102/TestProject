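; BP_Enemy is a GAS-based enemy character that can shoot, wander and take damage.
; BeginPlay sets an overhead widget fed by its AbilitySystemComponent and, if ShouldFire, starts a looping timer; Shoot activates BP_GA_Shoot.
; RandomPointMovement moves to random navigable points, pausing between moves.
; Damage applies BP_GE_GetDamage from the instigator's ability system, passing the amount via a SetByCaller tag.
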(event Custom|RandomPointMovement
  ;[0.1052 0.1052 0.1052] Moving to random point
  (bind (_randomlocation _returnvalue) (Class|NavigationSystemV1|GetRandomLocationinNavigableRadius (Transformation|GetActorLocation) 1e+04 0 0))
  (if _returnvalue
    (AI|AIMoveTo self _randomlocation 0 5.0 false
      (:OnSuccess
        _)
      (:OnFail
        _))
    (Utilities|FlowControl|Delay 3.0)
    (CallFunction|RandomPointMovement)))

(event EventBeginPlay
  ;[0.1052 0.1052 0.1052] Begin play
  (if (Variables|Default|GetbShouldFire)
    (bind _returnvalue (Utilities|Time|SetTimerbyEvent (EventDispatchers|CreateEvent :!event Shoot) 1.0 true))
    (Variables|Default|SetShootTimerH _returnvalue))
  (bind _returnvalue_2 (UserInterface|CreateWidget "/Game/Core/UI/NPCWidgets/WBP_OverheadWidget.WBP_OverheadWidget_C" (Game|GetPlayerController 0) (Variables|Default|GetAbilitySystemComponent)))
  (UserInterface|SetWidget (Variables|Default|GetWidget) _returnvalue_2))

(event EventDamage
  (params (DamageInstigator :type GAS%20Character%20Object%20Reference) (Hit :type Hit%20Result%20Structure%20%28by%20ref%29) (Damage :type Float%20%28single-precision%29))
  (bind _abilitysystemcomponent (Variables|/Script/Test.GASCharacter|GetAbilitySystemComponent DamageInstigator))
  (bind _returnvalue (Ability|GameplayEffect|AssignTagSetbyCallerMagnitude (GameplayEffects|MakeOutgoingSpec :self _abilitysystemcomponent :GameplayEffectClass "/Game/Core/GAS/GameplayEffects/Health/BP_GE_GetDamage.BP_GE_GetDamage_C" :Level 1.0) "(TagName=\"Attribute.BaseDamage\")" Damage))
  (GameplayEffects|ApplyGameplayEffectSpecToTarget _abilitysystemcomponent _returnvalue (Variables|Default|GetAbilitySystemComponent)))

(fn ConstructionScript)

(fn Shoot
  (Abilities|TryActivateAbilitybyClass (Variables|Default|GetAbilitySystemComponent) "/Game/Core/GAS/Abilities/CharacterSpecific/Common/BP_GA_Shoot.BP_GA_Shoot_C" true))